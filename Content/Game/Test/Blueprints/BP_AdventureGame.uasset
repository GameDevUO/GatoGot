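; BP_AdventureGame is a test camera actor for an orthographic side-on view that becomes player 0's view target on BeginPlay.
; The construction script sizes a CameraConfines box from ConfinesExtent.
; Get Camera Confines converts that box's X/Z bounds into min/max limits, inset by ortho-width fractions (half horizontally, 1/3.5 vertically).
; The limits are only stored here; Tick has no movement or clamping logic.
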(event `self.ReceiveBeginPlay`
  (`PlayerController.SetViewTargetWithBlend` (`GameplayStatics.GetPlayerController` 0) self 0.0 "VTBlend_Linear" 0.0 false)
  (`self.Get Camera Confines`
    (:`Out`
      (`KismetSystemLibrary.Delay` 0.0))))

(event `self.ReceiveTick`
  (params (DeltaSeconds :type "Float (single-precision)"))
  (set `self.Delta Seconds` DeltaSeconds))

(fn `UserConstructionScript`
  (`BoxComponent.SetBoxExtent` (`self.CameraConfines`) (`self.Confines Extent`) true))